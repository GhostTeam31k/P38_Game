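; Player-flyable P-38 plane pawn that flies forward constantly, with pitch and roll controls, rocket fire and a speed boost.
; FloatingPawnMovement drives forward motion every tick at the Velocity setting, while axis inputs apply frame-rate-scaled local rotations.
; A rotate component spins both propellers.
; Fire spawns a faster, short-lived BP_Rocket, and holding Boost doubles max speed with attached spark particles.
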(event EventBeginPlay
  (Utilities|Array|Add (Variables|/Game/P38/Actors/AC_RotateSceneComponents.AC_RotateSceneComponents_C|GetSceneComponents (Variables|Default|GetAC_RotateComponents)) (Variables|Default|GetSM_P38_Propeller_Right))
  (Utilities|Array|Add (Variables|/Game/P38/Actors/AC_RotateSceneComponents.AC_RotateSceneComponents_C|GetSceneComponents (Variables|Default|GetAC_RotateComponents)) (Variables|Default|GetSM_P38_Propeller_Left))
  (Variables|/Script/Engine.FloatingPawnMovement|SetMaxSpeed (Variables|Default|GetFloatingPawnMovement) (Variables|Movement|GetVelocity))
  (Variables|/Script/Engine.FloatingPawnMovement|SetAcceleration (Variables|Default|GetFloatingPawnMovement) (Variables|Movement|GetVelocity))
  (Variables|/Script/Engine.FloatingPawnMovement|SetDeceleration (Variables|Default|GetFloatingPawnMovement) (Variables|Movement|GetVelocity)))

(event EventTick
  (params (DeltaSeconds :type Float%20%28single-precision%29))
  (Pawn|Input|AddMovementInput (Transformation|GetActorForwardVector) 1.0 false))

(event Input|ActionEvents|InputActionFire
  (params (Key :type Key%20Structure))
  (:Pressed
    (Game|SpawnActorfromClass "/Game/Rocket/Actors/BP_Rocket.BP_Rocket_C" (Transformation|GetActorTransform) "Undefined" "MultiplyWithRoot" 0 (* (Variables|Movement|GetVelocity) 4.0) 3.0 0)))

(event Input|ActionEvents|InputActionBoost
  (params (Key :type Key%20Structure))
  (:Pressed
    (Variables|/Script/Engine.FloatingPawnMovement|SetMaxSpeed (Variables|Default|GetFloatingPawnMovement) (* (Variables|Movement|GetVelocity) 2.0))
    (bind _returnvalue (Effects|SpawnEmitterAttached "/Game/StarterContent/Particles/P_Sparks.P_Sparks" (Variables|Default|GetSM_P38_Body) "None"))
    (Variables|Default|SetSpark _returnvalue))
  (:Released
    (Variables|/Script/Engine.FloatingPawnMovement|SetMaxSpeed (Variables|Default|GetFloatingPawnMovement) (Variables|Movement|GetVelocity))
    (Components|DestroyComponent (Variables|Default|GetSpark))))

(event Input|AxisEvents|InputAxisPitch
  (params (AxisValue :type Float%20%28single-precision%29))
  (Transformation|AddActorLocalRotation (Math|Rotator|MakeRotator 0.0 (* AxisValue (Variables|Rotation|GetRotationVelocity) (Utilities|Time|GetWorldDeltaSeconds)) 0.0) false false))

(event Input|AxisEvents|InputAxisRoll
  (params (AxisValue :type Float%20%28single-precision%29))
  (Transformation|AddActorLocalRotation (Math|Rotator|MakeRotator (* AxisValue (Variables|Rotation|GetRotationVelocity) (Utilities|Time|GetWorldDeltaSeconds)) 0.0 0.0) false false))

(fn ConstructionScript)